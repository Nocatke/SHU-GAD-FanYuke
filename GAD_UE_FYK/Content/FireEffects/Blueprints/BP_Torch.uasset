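; BP_Torch is a configurable torch effect actor with optional mesh, smoke, light and distortion.
; The construction script hides components according to the Include flags, and disabling the light hides both the Rotator hierarchy and Distortion, regardless of the distortion flag.
; Each tick adds small sine-driven rotation deltas to Rotator, using a different frequency per axis to produce an irregular wobble.
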(event `self.ReceiveTick`
  (params (DeltaSeconds :type "Float (single-precision)"))
  (bind _returnvalue (`KismetSystemLibrary.GetGameTimeInSeconds`))
  (`SceneComponent.AddRelativeRotation` (`self.Rotator`) (`KismetMathLibrary.MakeRot` (`KismetMathLibrary.Sin` _returnvalue) (`KismetMathLibrary.Sin` (* _returnvalue 3.0)) (`KismetMathLibrary.Sin` (* _returnvalue 7.0))) false))

(fn `UserConstructionScript`
  (if (not (`self.IncludeSmoke`))
    (`SceneComponent.SetVisibility` (`self.TorchSmoke`) false false))
  (if (not (`self.IncludeMesh`))
    (`SceneComponent.SetVisibility` (`self.TorchMesh`) false false))
  (if (`self.IncludeLight`)
    (if (not (`self.IncludeDistortion`))
      (`SceneComponent.SetVisibility` (`self.Distortion`) false true :!label _label))
    (else
      (`SceneComponent.SetVisibility` (`self.Rotator`) false true)
      (goto _label))))